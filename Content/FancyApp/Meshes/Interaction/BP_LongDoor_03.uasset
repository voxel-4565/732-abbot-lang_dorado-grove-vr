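; BP_LongDoor_03 is an interactive door that toggles open and closed when its GrabComponent is grabbed.
; Each grab checks whether the stored right-side value is zero, then plays or reverses the Swing timeline accordingly.
; The timeline updates that value and uses it to rotate the kitchen door mesh up to 90 degrees in yaw.
; An unconnected relative-location node is unused.
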(event OnGrabbed(GrabComponent)
  (params (MotionController :type Motion%20Controller%20Component%20Object%20Reference))
  (Variables|Default|SetIsClosed_Right (== (Variables|Default|GetCurrentValue_Right) 0.0))
  (if (Variables|Default|GetIsClosed_Right)
    (bind _newtrack_0 (Timeline|Swing Play)
      (:Update
        (bind _output_get (Variables|Default|SetCurrentValue_Right _newtrack_0))
        (Transformation|SetRelativeRotation (Variables|Default|GetSM_DoorKitchen_01) (Math|Rotator|MakeRotator 0.0 0.0 (* _output_get 9e+01)) false false)))
    (else
      (Timeline|Swing Reverse))))

(fn ConstructionScript)