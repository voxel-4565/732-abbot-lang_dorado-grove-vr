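; BP_LongDoor_05 is a VR-grabbable kitchen door that swings open or closed on its yaw when grabbed.
; Inside and outside trigger boxes gate two timelines with identical swing direction, playing or reversing according to CurrentValueRight.
; BoxInside only ever sets InInside false, so in this graph only the outside box enables the swing.
; Another box briefly shows a hint widget to the VRPawn; leftover swing-direction logic is unconnected.
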(event OnComponentBeginOverlap(Box)
  (params (OverlappedComponent :type Primitive%20Component%20Object%20Reference) (OtherActor :type Actor%20Object%20Reference) (OtherComp :type Primitive%20Component%20Object%20Reference) (OtherBodyIndex :type Integer) (bFromSweep :type Boolean) (SweepResult :type Hit%20Result%20Structure%20%28by%20ref%29))
  ;[0.15 0.15 0.15 0.5] ShowHint
  (Utilities|Casting|CastToVRPawn OtherActor)
  (Class|WidgetComponent|SetTintColorandOpacity (Variables|Default|GetWidget) "(R=0.000000,G=0.000000,B=0.000000,A=1.000000)")
  (Utilities|FlowControl|Delay 1e+01)
  (Class|WidgetComponent|SetTintColorandOpacity (Variables|Default|GetWidget) "(R=1.000000,G=1.000000,B=1.000000,A=0.000000)"))

(event OnComponentEndOverlap(Box)
  (params (OverlappedComponent :type Primitive%20Component%20Object%20Reference) (OtherActor :type Actor%20Object%20Reference) (OtherComp :type Primitive%20Component%20Object%20Reference) (OtherBodyIndex :type Integer))
  ;[0.15 0.15 0.15 0.5] ShowHint
  (Utilities|Casting|CastToVRPawn OtherActor)
  (Class|WidgetComponent|SetTintColorandOpacity (Variables|Default|GetWidget) "(R=1.000000,G=1.000000,B=1.000000,A=0.000000)"))

(event OnComponentBeginOverlap(BoxInside)
  (params (OverlappedComponent :type Primitive%20Component%20Object%20Reference) (OtherActor :type Actor%20Object%20Reference) (OtherComp :type Primitive%20Component%20Object%20Reference) (OtherBodyIndex :type Integer) (bFromSweep :type Boolean) (SweepResult :type Hit%20Result%20Structure%20%28by%20ref%29))
  (Utilities|Casting|CastToVRPawn OtherActor)
  (Variables|Default|SetbInInside false))

(event OnGrabbed(GrabComponent)
  (params (MotionController :type Motion%20Controller%20Component%20Object%20Reference))
  (if (Variables|Default|GetbInInside)
    (Variables|Default|SetIsClosed_Right (== (Variables|Default|GetCurrentValue_Right) 0.0))
    (if (Variables|Default|GetIsClosed_Right)
      (bind _newtrack_0 (Timeline|Timeline Play)
        (:Update
          (bind _output_get (Variables|Default|SetCurrentValue_Right _newtrack_0))
          (Transformation|SetRelativeRotation (Variables|Default|GetSM_DoorKitchen_01) (Math|Rotator|MakeRotator 0.0 0.0 (* _output_get -9e+01)) false false)))
      (else
        (Timeline|Timeline Reverse)))
    (elif (Variables|Default|GetbOnOutside)
      (Variables|Default|SetIsClosed_Right (== (Variables|Default|GetCurrentValue_Right) 0.0))
      (if (Variables|Default|GetIsClosed_Right)
        (bind _newtrack_0_2 (Timeline|Timeline_0 Play)
          (:Update
            (bind _output_get_2 (Variables|Default|SetCurrentValue_Right _newtrack_0_2))
            (Transformation|SetRelativeRotation (Variables|Default|GetSM_DoorKitchen_01) (Math|Rotator|MakeRotator 0.0 0.0 (* _output_get_2 -9e+01)) false false)))
        (else
          (Timeline|Timeline_0 Reverse))))))

(event OnComponentEndOverlap(BoxInside)
  (params (OverlappedComponent :type Primitive%20Component%20Object%20Reference) (OtherActor :type Actor%20Object%20Reference) (OtherComp :type Primitive%20Component%20Object%20Reference) (OtherBodyIndex :type Integer))
  (Utilities|Casting|CastToVRPawn OtherActor)
  (Variables|Default|SetbInInside false))

(event OnComponentBeginOverlap(BoxOutside)
  (params (OverlappedComponent :type Primitive%20Component%20Object%20Reference) (OtherActor :type Actor%20Object%20Reference) (OtherComp :type Primitive%20Component%20Object%20Reference) (OtherBodyIndex :type Integer) (bFromSweep :type Boolean) (SweepResult :type Hit%20Result%20Structure%20%28by%20ref%29))
  (Utilities|Casting|CastToVRPawn OtherActor)
  (Variables|Default|SetbOnOutside true))

(event OnComponentEndOverlap(BoxOutside)
  (params (OverlappedComponent :type Primitive%20Component%20Object%20Reference) (OtherActor :type Actor%20Object%20Reference) (OtherComp :type Primitive%20Component%20Object%20Reference) (OtherBodyIndex :type Integer))
  (Utilities|Casting|CastToVRPawn OtherActor)
  (Variables|Default|SetbOnOutside false))

(fn ConstructionScript)