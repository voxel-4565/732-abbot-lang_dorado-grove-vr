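; VR kitchen door that swings to plus or minus 90 degrees yaw when grabbed, depending on whether the VRPawn is in the inside trigger box.
; A Swing timeline lerps the yaw, with a busy flag blocking grabs mid-swing.
; No path closes it: open and closed branches are identical.
; A third box shows a hint widget, hidden on exit or after a delay; outside-box tracking feeds only unreachable debug code.
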(event OnComponentBeginOverlap(Box)
  (params (OverlappedComponent :type Primitive%20Component%20Object%20Reference) (OtherActor :type Actor%20Object%20Reference) (OtherComp :type Primitive%20Component%20Object%20Reference) (OtherBodyIndex :type Integer) (bFromSweep :type Boolean) (SweepResult :type Hit%20Result%20Structure%20%28by%20ref%29))
  ;[0.15 0.15 0.15 0.5] ShowHint
  (Utilities|Casting|CastToVRPawn OtherActor)
  (Class|WidgetComponent|SetTintColorandOpacity (Variables|Default|GetWidget) "(R=0.000000,G=0.000000,B=0.000000,A=1.000000)")
  (Utilities|FlowControl|Delay 1e+01)
  (Class|WidgetComponent|SetTintColorandOpacity (Variables|Default|GetWidget) "(R=1.000000,G=1.000000,B=1.000000,A=0.000000)"))

(event OnComponentEndOverlap(Box)
  (params (OverlappedComponent :type Primitive%20Component%20Object%20Reference) (OtherActor :type Actor%20Object%20Reference) (OtherComp :type Primitive%20Component%20Object%20Reference) (OtherBodyIndex :type Integer))
  ;[0.15 0.15 0.15 0.5] ShowHint
  (Utilities|Casting|CastToVRPawn OtherActor)
  (Class|WidgetComponent|SetTintColorandOpacity (Variables|Default|GetWidget) "(R=1.000000,G=1.000000,B=1.000000,A=0.000000)"))

(event OnComponentEndOverlap(BoxOutside)
  (params (OverlappedComponent :type Primitive%20Component%20Object%20Reference) (OtherActor :type Actor%20Object%20Reference) (OtherComp :type Primitive%20Component%20Object%20Reference) (OtherBodyIndex :type Integer))
  (Utilities|Casting|CastToVRPawn OtherActor)
  (Variables|Default|SetbInOutside false))

(event OnComponentBeginOverlap(BoxInside)
  (params (OverlappedComponent :type Primitive%20Component%20Object%20Reference) (OtherActor :type Actor%20Object%20Reference) (OtherComp :type Primitive%20Component%20Object%20Reference) (OtherBodyIndex :type Integer) (bFromSweep :type Boolean) (SweepResult :type Hit%20Result%20Structure%20%28by%20ref%29))
  (Utilities|Casting|CastToVRPawn OtherActor)
  (Variables|Default|SetbInInside true))

(event OnGrabbed(GrabComponent)
  (params (MotionController :type Motion%20Controller%20Component%20Object%20Reference))
  (if (not (Variables|Default|GetbIsBusy))
    (Variables|Default|SetbIsBusy true)
    (if (Variables|Default|GetbIsOpen)
      ;[0.15 0.15 0.15 0.5] IsOpenTrue
      (if (Variables|Default|GetbInInside)
        (bind _output_get (Variables|Default|SetOpenYaw -9e+01))
        (Variables|Default|SetLastOpenYaw _output_get)
        (CallFunction|DoOpenDoor)
        (else
          (bind _output_get_2 (Variables|Default|SetOpenYaw 9e+01))
          (Variables|Default|SetLastOpenYaw _output_get_2)
          (CallFunction|DoOpenDoor)))
      (else
        ;[0.15 0.15 0.15 0.5] IsOpenFalse
        (if (Variables|Default|GetbInInside)
          (bind _output_get_3 (Variables|Default|SetOpenYaw -9e+01))
          (Variables|Default|SetLastOpenYaw _output_get_3)
          (CallFunction|DoOpenDoor)
          (else
            (bind _output_get_4 (Variables|Default|SetOpenYaw 9e+01))
            (Variables|Default|SetLastOpenYaw _output_get_4)
            (CallFunction|DoOpenDoor)))))))

(event OnComponentEndOverlap(BoxInside)
  (params (OverlappedComponent :type Primitive%20Component%20Object%20Reference) (OtherActor :type Actor%20Object%20Reference) (OtherComp :type Primitive%20Component%20Object%20Reference) (OtherBodyIndex :type Integer))
  (Utilities|Casting|CastToVRPawn OtherActor)
  (Variables|Default|SetbInInside false))

(event OnComponentBeginOverlap(BoxOutside)
  (params (OverlappedComponent :type Primitive%20Component%20Object%20Reference) (OtherActor :type Actor%20Object%20Reference) (OtherComp :type Primitive%20Component%20Object%20Reference) (OtherBodyIndex :type Integer) (bFromSweep :type Boolean) (SweepResult :type Hit%20Result%20Structure%20%28by%20ref%29))
  (Utilities|Casting|CastToVRPawn OtherActor)
  (Variables|Default|SetbInOutside true))

(event Custom|DoOpenDoor
  (Variables|Default|SetbIsOpen true)
  (Components|Timeline|SetPlayRate (Variables|Default|GetSwing) (/ 1.0 (Variables|Default|GetOpenDuration)))
  (Variables|Default|SetStartYaw (.Yaw (Math|Rotator|BreakRotator (Variables|/Script/Engine.SceneComponent|GetRelativeRotation (Variables|Default|GetSM_DoorKitchen_01)))))
  (Variables|Default|SetTargetYaw (Variables|Default|GetOpenYaw))
  (bind _alpha (Timeline|Swing PlayFromStart)
    (:Update
      (Transformation|SetRelativeRotation (Variables|Default|GetSM_DoorKitchen_01) (Math|Rotator|MakeRotator 0.0 0.0 (Math|Float|Lerp (Variables|Default|GetStartYaw) (Variables|Default|GetTargetYaw) _alpha)) false false))
    (:Finished
      (Variables|Default|SetbIsBusy false))))

(fn ConstructionScript)