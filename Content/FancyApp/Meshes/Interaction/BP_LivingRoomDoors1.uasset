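; VR living room sliding door Blueprint that lets a motion controller move the right door by grabbing it.
; A grab within the right collision sphere's radius starts a short timer whose event sets the door's world Y to the controller's, keeping its initial X and Z.
; Dropping clears the controller reference and calls pause on the timer by function name.
; The left grab handler only checks range and moves nothing.
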(event OnGrabbed(GrabComponent_Right)
  (params (MotionController :type Motion%20Controller%20Component%20Object%20Reference))
  (bind _spherecollision_right (Variables|Default|GetSphereCollision_Right))
  (Utilities|IsValid MotionController
    (:Is%20Valid
      (bind _output_get (Variables|Default|SetMotion%20Controller MotionController))
      (if (Utilities|Operators|EqualEqual (Transformation|GetWorldLocation _output_get) (Transformation|GetWorldLocation _spherecollision_right) (Variables|/Script/Engine.SphereComponent|GetSphereRadius _spherecollision_right))
        (Utilities|Time|SetTimerbyEvent (delegate Custom|EventRightDoor) 0.1)))))

(event OnGrabbed(GrabComponent_Left)
  (params (MotionController :type Motion%20Controller%20Component%20Object%20Reference))
  (bind _spherecollision_left (Variables|Default|GetSphereCollision_Left))
  (if (Utilities|Operators|EqualEqual (Transformation|GetWorldLocation MotionController) (Transformation|GetWorldLocation _spherecollision_left) (Variables|/Script/Engine.SphereComponent|GetSphereRadius _spherecollision_left))
    _))

(event OnDropped(GrabComponent_Right)
  (Variables|Default|SetMotion%20Controller 0)
  (Class|KismetSystemLibrary|PauseTimer 0 "EventRightDoor"))

(event Custom|EventRightDoor
  (bind _initiallocationrightdoor (Variables|Default|GetInitialLocationRightDoor))
  (Transformation|SetWorldLocation (Variables|Default|GetSM_LivingDoor_Right_01) (Math|Vector|MakeVector (.x _initiallocationrightdoor) (.y (Transformation|GetWorldLocation (Variables|Default|GetMotion%20Controller))) (.z _initiallocationrightdoor)) false false))

(event EventBeginPlay
  (Variables|Default|SetInitialLocationRightDoor (Transformation|GetWorldLocation (Variables|Default|GetSM_LivingDoor_Right_01))))

(fn ConstructionScript)