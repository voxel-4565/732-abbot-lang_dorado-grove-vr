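; Interactive single door Blueprint that opens and closes when its right-side grab component is grabbed.
; A grab while closed tilts the handle mesh via one timeline, then after a short delay swings the door up to 90 degrees via a second timeline.
; A grab at any other door value reverses both timelines, and both directions play the same 2D door sound.
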(event OnGrabbed(GrabComponent_Right)
  (params (MotionController :type Motion%20Controller%20Component%20Object%20Reference))
  (Variables|Default|SetIsClosed_Right (== (Variables|Default|GetCurrentValue_Right) 0.0))
  (if (Variables|Default|GetIsClosed_Right)
    (Utilities|FlowControl|Sequence
      (:then_0
        (bind _newtrack_0 (Timeline|Timeline Play)
          (:Update
            (Transformation|SetRelativeRotation (Variables|Default|GetHandleMesh_Right) (Math|Rotator|MakeRotator (Math|Float|Lerp 0.0 -2e+01 _newtrack_0) 0.0 0.0) false false))))
      (:then_1
        (Utilities|FlowControl|Delay 0.66)
        (bind _newtrack_0_2 (Timeline|Timeline_1 Play)
          (:Update
            (bind _output_get (Variables|Default|SetCurrentValue_Right _newtrack_0_2))
            (Transformation|SetRelativeRotation (Variables|Default|GetSM_LivingDoor_Right_01) (Math|Rotator|MakeRotator 0.0 0.0 (* _output_get 9e+01)) false false))))
      (:then_2
        (Audio|PlaySound2D "/Game/FancyApp/Sounds/opening-door-411632.opening-door-411632" 1.0 1.0 0.0 0 0)))
    (else
      (Utilities|FlowControl|Sequence
        (:then_0
          (Timeline|Timeline Reverse))
        (:then_1
          (Timeline|Timeline_1 Reverse))
        (:then_2
          (Audio|PlaySound2D "/Game/FancyApp/Sounds/opening-door-411632.opening-door-411632" 1.0 1.0 0.0 0 0))))))

(fn ConstructionScript)