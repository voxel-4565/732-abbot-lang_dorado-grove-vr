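; Planar mirror actor prototype built on a SceneCaptureComponent2D, which hides its own Plane from the capture on BeginPlay.
; Tick only stores the mirror transform, the camera forward in mirror space and LocalCamPos, which uses the mirror root's location instead of the camera's.
; Nothing live moves the capture: UpdateMirror is empty, and the reflection-vector placement, timer, timeline and debug prints are disconnected experiments.
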(event Custom|UpdateMirror)

(event EventBeginPlay
  (Class|SceneCaptureComponent|HideComponent (Variables|Default|GetSceneCaptureComponent2D) (Variables|Default|GetPlane)))

(event EventTick
  (params (DeltaSeconds :type Float%20%28single-precision%29))
  (bind _mirrorplaneroot (Variables|Default|GetMirrorPlaneRoot))
  (bind _output_get (Variables|Default|SetMirrorTM (Transformation|GetWorldTransform _mirrorplaneroot)))
  (bind _output_get_2 (Variables|Default|SetLocalCamPos (Math|Transform|InverseTransformLocation _output_get (Transformation|GetWorldLocation _mirrorplaneroot))))
  (bind _output_get_3 (Variables|Default|SetLocalCamForward (Math|Transform|InverseTransformDirection _output_get (Math|Vector|GetForwardVector (Camera|GetCameraRotation (Game|GetPlayerCameraManager 0)))))))

(fn ConstructionScript)