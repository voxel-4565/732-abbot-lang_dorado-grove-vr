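; Mirror actor for a living room that fakes a planar reflection with a SceneCaptureComponent2D, which hides the mirror Plane from its own capture.
; Each tick it reflects the view target's camera position and axes about the actor's forward vector to place and orient the capture.
; The result gets a fixed correction: negated world Y on the location and a half-turn of yaw on the rotation.
; Timeline, timer and UpdateMirror are inactive leftovers.
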(event Custom|UpdateMirror)

(event EventBeginPlay
  (Class|SceneCaptureComponent|HideComponent (Variables|Default|GetSceneCaptureComponent2D) (Variables|Default|GetPlane)))

(event EventTick
  (params (DeltaSeconds :type Float%20%28single-precision%29))
  (bind _returnvalue (Game|GetPlayerController 0))
  (bind _returnvalue_2 (Transformation|GetActorForwardVector))
  (bind _scenecapturecomponent2d (Variables|Default|GetSceneCaptureComponent2D))
  (bind _plane (Variables|Default|GetPlane))
  (bind _returnvalue_3 (Pawn|GetViewTarget _returnvalue))
  (bind _returnvalue_4 (Utilities|IsValid _scenecapturecomponent2d))
  (bind _returnvalue_5 (Transformation|GetWorldLocation _plane))
  (bind _returnvalue_6 (Actor|GetComponentsByClass _returnvalue_3 "/Script/Engine.CameraComponent"))
  (bind _output (Utilities|Array|Get(acopy) _returnvalue_6))
  (bind _returnvalue_7 (Transformation|GetWorldLocation _output))
  (bind _returnvalue_8 (- _returnvalue_5 _returnvalue_7))
  (bind _returnvalue_9 (Math|Vector|GetReflectionVector _returnvalue_8 _returnvalue_2))
  (bind _returnvalue_10 (* _returnvalue_9 -1.0))
  (bind _returnvalue_11 (+ _returnvalue_5 _returnvalue_10))
  (if (and (!= (Utilities|Array|Length _returnvalue_6) 0) _returnvalue_4)
    (Transformation|SetWorldLocation _scenecapturecomponent2d (Math|Vector|MakeVector (.x _returnvalue_11) (* (.y _returnvalue_11) -1.0) (.z _returnvalue_11)) false false)
    (Transformation|SetWorldRotation _scenecapturecomponent2d (Math|Rotator|CombineRotators (Math|Rotator|MakeRotfromXY (Math|Vector|GetReflectionVector (Math|Vector|GetForwardVector _output) _returnvalue_2) (* (Math|Vector|GetReflectionVector (Math|Vector|GetRightVector _output) _returnvalue_2) -1.0)) (Math|Rotator|MakeRotator 0.0 0.0 1.8e+02)) false false)
    (elif (not _returnvalue_4)
      (Development|PrintString "Hello"))))

(fn ConstructionScript)