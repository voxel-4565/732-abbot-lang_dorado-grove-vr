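; Mirror actor that drives a SceneCaptureComponent2D from the player's view to fake a planar reflection.
; A looping timer started on BeginPlay reflects the view target's camera offset from the Plane across the actor's forward vector to position the capture.
; The resulting world Y is negated, and capture rotation copies the camera's unmirrored, leaving a reflected-rotation calculation unused.
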(event Custom|UpdateMirror
  (bind _returnvalue (Game|GetPlayerController 0))
  (bind _returnvalue_2 (Transformation|GetActorForwardVector))
  (bind _scenecapturecomponent2d (Variables|Default|GetSceneCaptureComponent2D))
  (bind _plane (Variables|Default|GetPlane))
  (bind _returnvalue_3 (Pawn|GetViewTarget _returnvalue))
  (bind _returnvalue_4 (Utilities|IsValid _scenecapturecomponent2d))
  (bind _returnvalue_5 (Transformation|GetWorldLocation _plane))
  (bind _returnvalue_6 (Actor|GetComponentsByClass _returnvalue_3 "/Script/Engine.CameraComponent"))
  (bind _output (Utilities|Array|Get(acopy) _returnvalue_6))
  (bind _returnvalue_7 (Transformation|GetWorldLocation _output))
  (bind _returnvalue_8 (- _returnvalue_5 _returnvalue_7))
  (bind _returnvalue_9 (Math|Vector|GetReflectionVector _returnvalue_8 _returnvalue_2))
  (bind _returnvalue_10 (* _returnvalue_9 -1.0))
  (bind _returnvalue_11 (+ _returnvalue_5 _returnvalue_10))
  (if (and (!= (Utilities|Array|Length _returnvalue_6) 0) _returnvalue_4)
    (Transformation|SetWorldLocation _scenecapturecomponent2d (Math|Vector|MakeVector (.x _returnvalue_11) (* (.y _returnvalue_11) -1.0) (.z _returnvalue_11)) false false)
    (Transformation|SetWorldRotation _scenecapturecomponent2d (Transformation|GetWorldRotation _output) false false)
    (elif (not _returnvalue_4)
      (Development|PrintString "Hello"))))

(event EventBeginPlay
  (Utilities|Time|SetTimerbyEvent (delegate Custom|UpdateMirror) 0.05 true))

(fn ConstructionScript)