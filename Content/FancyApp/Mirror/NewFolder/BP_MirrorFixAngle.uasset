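; Mirror actor that drives a SceneCaptureComponent2D as a planar reflection of the player's view.
; Each Tick it takes the first camera component on player 0's view target and mirrors its position across the plane through the root, using the actor's forward vector as normal.
; Capture rotation is rebuilt from the reflected forward and negated reflected right vectors.
; An invalid capture component only prints a debug string.
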(event EventTick
  (params (DeltaSeconds :type Float%20%28single-precision%29))
  (bind _returnvalue (Game|GetPlayerController 0))
  (bind _returnvalue_2 (Transformation|GetActorForwardVector))
  (bind _self self)
  (bind _scenecapturecomponent2d (Variables|Default|GetSceneCaptureComponent2D))
  (bind _returnvalue_3 (Pawn|GetViewTarget _returnvalue))
  (bind _returnvalue_4 (Utilities|IsValid _scenecapturecomponent2d))
  (bind _defaultsceneroot (Variables|Default|GetDefaultSceneRoot _self))
  (bind _returnvalue_5 (Actor|GetComponentsByClass _returnvalue_3 "/Script/Engine.CameraComponent"))
  (bind _returnvalue_6 (Transformation|GetWorldLocation _defaultsceneroot))
  (bind _output (Utilities|Array|Get(acopy) _returnvalue_5))
  (if (and (!= (Utilities|Array|Length _returnvalue_5) 0) _returnvalue_4)
    (Transformation|SetWorldLocation _scenecapturecomponent2d (+ _returnvalue_6 (* (Math|Vector|GetReflectionVector (- _returnvalue_6 (Transformation|GetWorldLocation _output)) _returnvalue_2) -1.0)) false false)
    (Transformation|SetWorldRotation _scenecapturecomponent2d (Math|Rotator|MakeRotfromXY (Math|Vector|GetReflectionVector (Math|Vector|GetForwardVector _output) _returnvalue_2) (* (Math|Vector|GetReflectionVector (Math|Vector|GetRightVector _output) _returnvalue_2) -1.0)) false false)
    (elif (not _returnvalue_4)
      (Development|PrintString "Hello"))))

(fn ConstructionScript)