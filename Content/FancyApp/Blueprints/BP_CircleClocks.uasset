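; BP_CircleClocks is an analog wall-style clock actor that shows the current real-world time and ticks audibly.
; A looping one-second timer started on BeginPlay calls UpdateAnalogClock, which sets the yaw of the hour, minute and second arrows from Now().
; The hour hand advances gradually with the minutes.
; An attenuated tick-tock sound plays at the clock base whenever the stored second changes.
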(event EventBeginPlay
  (Utilities|Time|SetTimerbyFunctionName 0 "UpdateAnalogClock" 1.0 true))

(fn ConstructionScript)

(fn UpdateAnalogClock
  (bind _returnvalue (Math|DateTime|Now))
  (bind (_year _month _day _hour _minute _second) (Math|DateTime|BreakDateTime _returnvalue))
  (Transformation|SetRelativeRotation (Variables|Default|GetArrow_Hour) (Math|Rotator|MakeRotator 0.0 0.0 (Math|Conversions|ToFloat(Integer) (+ (* (Math|Integer|%(Integer) _hour 12) 30) (* _minute 0.5)))) false false)
  (Transformation|SetRelativeRotation (Variables|Default|GetArrow_Min) (Math|Rotator|MakeRotator 0.0 0.0 (Math|Conversions|ToFloat(Integer) (* _minute 6))) false false)
  (Transformation|SetRelativeRotation (Variables|Default|GetArrow_Second) (Math|Rotator|MakeRotator 0.0 0.0 (Math|Conversions|ToFloat(Integer) (* _second 6))) false false)
  (if (!= _second (Variables|Default|GetLastTickSecond))
    (Audio|PlaySoundatLocation "/Game/FancyApp/Audio/MSS_TicTac.MSS_TicTac" (.Location (Math|Transform|BreakTransform (Transformation|GetWorldTransform (Variables|Default|GetSM_ClocksBase)))) "0, 0, 0" 0.5 1.0 0.0 "/Game/FancyApp/Audio/NewSoundAttenuation.NewSoundAttenuation" 0 0 0)
    (Variables|Default|SetLastTickSecond _second)))