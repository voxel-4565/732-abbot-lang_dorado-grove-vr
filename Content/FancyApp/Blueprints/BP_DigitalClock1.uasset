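; Digital clock Blueprint that shows the system time on four digit planes with a blinking two-dot separator.
; BeginPlay creates a dynamic material per digit and starts a looping one-second timer.
; Each tick splits hour and minute into digits, swaps opacity textures from a digit array and toggles the dots on second parity.
; Hours use 12-hour format; enabling Is24HourFormat selects a constant 0, so hours show 00.
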(event EventBeginPlay
  (bind _returnvalue (Rendering|Material|CreateDynamicMaterialInstance (Variables|Default|GetPlane_Hour1) 0 0 "None" :!class /Script/Engine.PrimitiveComponent))
  (Variables|Default|SetDMI_Hour1 _returnvalue)
  (bind _returnvalue_2 (Rendering|Material|CreateDynamicMaterialInstance (Variables|Default|GetPlane_Hour2) 0 0 "None" :!class /Script/Engine.PrimitiveComponent))
  (Variables|Default|SetDMI_Hour2 _returnvalue_2)
  (bind _returnvalue_3 (Rendering|Material|CreateDynamicMaterialInstance (Variables|Default|GetPlane_Minute1) 0 0 "None" :!class /Script/Engine.PrimitiveComponent))
  (Variables|Default|SetDMI_MInute1 _returnvalue_3)
  (bind _returnvalue_4 (Rendering|Material|CreateDynamicMaterialInstance (Variables|Default|GetPlane_Minute2) 0 0 "None" :!class /Script/Engine.PrimitiveComponent))
  (Variables|Default|SetDMI_Minute2 _returnvalue_4)
  (Utilities|Time|SetTimerbyFunctionName 0 "UpdateClockTextures" 1.0 true))

(fn ConstructionScript)

(fn UpdateClockTextures
  (bind _returnvalue (Math|DateTime|Now))
  (bind _bis24hourformat (Variables|Default|GetbIs24HourFormat))
  (bind (_year _month _day _hour _minute _second) (Math|DateTime|BreakDateTime _returnvalue))
  (bind _returnvalue_2 (Math|Integer|%(Integer) _hour 12))
  (bind _returnvalue_3 (== _returnvalue_2 0))
  (bind _returnvalue_4 (Math|Integer|SelectInt 12 _returnvalue_2 _returnvalue_3))
  (bind _returnvalue_5 (Math|Integer|SelectInt 0 _returnvalue_4 _bis24hourformat))
  (Rendering|Material|SetTextureParameterValue (Variables|Default|GetDMI_Hour1) "OpacityTex" (Utilities|Array|Get(acopy) (Variables|Default|GetDigittexturesArray) (/ _returnvalue_5 10)))
  (Rendering|Material|SetTextureParameterValue (Variables|Default|GetDMI_Hour2) "OpacityTex" (Utilities|Array|Get(acopy) (Variables|Default|GetDigittexturesArray) (Math|Integer|%(Integer) _returnvalue_5 10)))
  (Rendering|Material|SetTextureParameterValue (Variables|Default|GetDMI_MInute1) "OpacityTex" (Utilities|Array|Get(acopy) (Variables|Default|GetDigittexturesArray) (/ _minute 10)))
  (Rendering|Material|SetTextureParameterValue (Variables|Default|GetDMI_Minute2) "OpacityTex" (Utilities|Array|Get(acopy) (Variables|Default|GetDigittexturesArray) (Math|Integer|%(Integer) _minute 10)))
  (Rendering|SetVisibility (Variables|Default|GetPlane_TwoDots) (== (Math|Integer|%(Integer) _second 2) 0) false))