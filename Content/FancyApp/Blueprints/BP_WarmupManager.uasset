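; Warmup manager actor that briefly takes over the player's view at level start to tour a BP_WarmupCamera through every TargetPoint.
; After a delay it blocks move and look input, then a repeating timer event teleports the camera point to point.
; In parallel, it hides the VRPawn's loading widget.
; When finished, it restores view and input and destroys warmup spheres, cameras and itself.
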(event Custom|Warmup_NextPoint
  (if (>= (Variables|Default|GetCurrentIndex) (Utilities|Array|Length (stale EventBeginPlay _output_get_2)))
    (CallFunction|WarmupFinish)
    (else
      (bind _output_get (Variables|Default|SetTargetPoint (Utilities|Array|Get(acopy) (stale EventBeginPlay _output_get_2) (Variables|Default|GetCurrentIndex))))
      (Transformation|SetActorTransform (Variables|Default|GetWarmupCamera) (Transformation|GetActorTransform _output_get) false true)
      (Game|Player|SetViewTargetwithBlend (Variables|Default|GetPlayerController) (Variables|Default|GetWarmupCamera) 0.2 "VTBlend_Linear" 0.0 false)
      (Variables|Default|SetCurrentIndex (+ (Variables|Default|GetCurrentIndex) 1))
      (Utilities|Time|SetTimerbyEvent (delegate Custom|Warmup_NextPoint) 2.0))))

(event Custom|Warmup_Finish
  (bind _returnvalue (Game|GetPlayerController 0))
  (Utilities|FlowControl|Delay 2.0)
  (Game|Player|SetViewTargetwithBlend (Variables|Default|GetPlayerController) (Variables|Default|GetOriginalViewTarget) 0.0 "VTBlend_Linear" 0.0 false)
  (Input|SetIgnoreMoveInput _returnvalue false)
  (Input|SetIgnoreLookInput _returnvalue false)
  (bind _outactors (Actor|GetAllActorsOfClass "/Game/FancyApp/Blueprints/BP_WarmupSphere.BP_WarmupSphere_C"))
  (Actor|DestroyActor _outactors)
  (bind _outactors_2 (Actor|GetAllActorsOfClass "/Game/FancyApp/Blueprints/BP_WarmupCamera.BP_WarmupCamera_C"))
  (Actor|DestroyActor _outactors_2)
  (Actor|DestroyActor))

(event EventBeginPlay
  (bind _returnvalue (Game|GetPlayerController 0))
  (bind _returnvalue_2 (Game|GetPlayerController 0))
  (Development|PrintString "CameraWarmupEnable" true true "(R=0.000000,G=0.660000,B=1.000000,A=1.000000)" 1.0)
  (Utilities|FlowControl|Sequence
    (:then_0
      (bind _outactors (Actor|GetAllActorsOfClass "/Game/FancyApp/Blueprints/BP_WarmupCamera.BP_WarmupCamera_C"))
      (bind _output_get (Variables|Default|SetWarmupCamera (Utilities|Array|Get(acopy) _outactors)))
      (Development|PrintString (Utilities|GetDisplayName _output_get) true true "(R=0.000000,G=0.456759,B=1.000000,A=1.000000)")
      (bind _outactors_2 (Actor|GetAllActorsOfClass "/Script/Engine.TargetPoint"))
      (bind _output_get_2 (Variables|Default|SetWarmupPoints _outactors_2))
      (Utilities|FlowControl|Delay 6.0)
      (Variables|Default|SetPlayerController _returnvalue_2)
      (Variables|Default|SetOriginalViewTarget (Pawn|GetViewTarget _returnvalue_2))
      (Input|SetIgnoreMoveInput _returnvalue true)
      (Input|SetIgnoreLookInput _returnvalue true)
      (Development|PrintString (Utilities|String|ToString(Integer) (Utilities|Array|Length _output_get_2)) true true "(R=1.000000,G=0.215178,B=0.063574,A=1.000000)" 1e+01)
      (Game|Player|SetViewTargetwithBlend (Variables|Default|GetPlayerController) (Variables|Default|GetWarmupCamera) 0.0 "VTBlend_Linear" 0.0 false)
      (CallFunction|WarmupNextPoint))
    (:then_1
      (Utilities|FlowControl|Delay 4.0)
      (bind _asvrpawn (Utilities|Casting|CastToVRPawn (Game|Player|GetPlayerPawn 0)))
      (Rendering|SetVisibility (Variables|/Game/VRTemplate/Blueprints/VRPawn.VRPawn_C|GetWidgetLoading _asvrpawn) false false))))

(fn ConstructionScript)