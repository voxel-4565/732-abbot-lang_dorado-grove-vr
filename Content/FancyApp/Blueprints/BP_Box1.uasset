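; VR two-drawer furniture piece whose top and bottom drawers are grabbed and slid with motion controllers.
; While a drawer is held, a fast looping timer moves it along local Y to follow the controller, clamped between two spline points.
; Sphere overlaps with tagged collision components trigger attenuated open and close sounds, gated by paired DoOnce nodes that reset each other.
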(event OnGrabbed(GrabComponent_Down)
  (params (MotionController :type Motion%20Controller%20Component%20Object%20Reference))
  ;[0.15 0.15 0.15 0.5] DownDrawerPart
  (Variables|Default|SetMotion%20Controller MotionController)
  (Utilities|FlowControl|Sequence
    (:then_0
      (bind _returnvalue (Utilities|Time|SetTimerbyFunctionName 0 "BoxDown" 0.01 true))
      (Variables|Default|SetTimerDown _returnvalue))))

(event OnGrabbed(GrabComponent_Top)
  (params (MotionController :type Motion%20Controller%20Component%20Object%20Reference))
  ;[0.15 0.15 0.15 0.5] TopDrawerPart
  (Variables|Default|SetMotion%20Controller MotionController)
  (Utilities|FlowControl|Sequence
    (:then_0
      (bind _returnvalue (Utilities|Time|SetTimerbyFunctionName 0 "BoxTopper" 0.01 true))
      (Variables|Default|SetTimerTop _returnvalue))))

(event OnComponentBeginOverlap(Sphere_Bottom)
  (params (OverlappedComponent :type Primitive%20Component%20Object%20Reference) (OtherActor :type Actor%20Object%20Reference) (OtherComp :type Primitive%20Component%20Object%20Reference) (OtherBodyIndex :type Integer) (bFromSweep :type Boolean) (SweepResult :type Hit%20Result%20Structure%20%28by%20ref%29))
  ;[0.15 0.15 0.15 0.5] TopDrawerPart_Sound
  (if (Components|ComponentHasTag OtherComp "BottomCollision")
    (Utilities|FlowControl|Sequence
      (:then_0
        (Utilities|FlowControl|DoOnce false
          (:Completed
            (Audio|PlaySoundatLocation "/Game/FancyApp/Audio/Open.Open" (Transformation|GetWorldLocation (Variables|Default|GetSM_RoomTumb_03)) "0, 0, 0" 1.0 1.0 0.0 "/Game/FancyApp/Audio/SA_Drawer.SA_Drawer" 0 0 0))))
      (:then_1
        (Utilities|FlowControl|DoOnce false) ; enters at Reset
      ))))

(event OnComponentEndOverlap(Sphere_Bottom)
  (params (OverlappedComponent :type Primitive%20Component%20Object%20Reference) (OtherActor :type Actor%20Object%20Reference) (OtherComp :type Primitive%20Component%20Object%20Reference) (OtherBodyIndex :type Integer))
  ;[0.15 0.15 0.15 0.5] TopDrawerPart_Sound
  (if (Components|ComponentHasTag OtherComp "BottomCollision")
    (Utilities|FlowControl|Sequence
      (:then_0
        (Utilities|FlowControl|DoOnce false
          (:Completed
            (Audio|PlaySoundatLocation "/Game/FancyApp/Audio/Close.Close" (Transformation|GetWorldLocation (Variables|Default|GetSM_RoomTumb_03)) "0, 0, 0" 1.0 1.0 0.0 "/Game/FancyApp/Audio/SA_Drawer.SA_Drawer" 0 0 0))))
      (:then_1
        (Utilities|FlowControl|DoOnce false) ; enters at Reset
      ))))

(event OnDropped(GrabComponent_Top)
  ;[0.15 0.15 0.15 0.5] TopDrawerPart
  (Utilities|Time|ClearandInvalidateTimerbyHandle (Variables|Default|GetTimerTop))
  (Variables|Default|SetMotion%20Controller 0))

(event OnDropped(GrabComponent_Down)
  ;[0.15 0.15 0.15 0.5] DownDrawerPart
  (Utilities|Time|ClearandInvalidateTimerbyHandle (Variables|Default|GetTimerDown))
  (Variables|Default|SetMotion%20Controller 0))

(event OnComponentBeginOverlap(Sphere_Top)
  (params (OverlappedComponent :type Primitive%20Component%20Object%20Reference) (OtherActor :type Actor%20Object%20Reference) (OtherComp :type Primitive%20Component%20Object%20Reference) (OtherBodyIndex :type Integer) (bFromSweep :type Boolean) (SweepResult :type Hit%20Result%20Structure%20%28by%20ref%29))
  ;[0.15 0.15 0.15 0.5] TopDrawerPart_Sound
  (if (Components|ComponentHasTag OtherComp "TopCollision")
    (Utilities|FlowControl|Sequence
      (:then_0
        (Utilities|FlowControl|DoOnce false
          (:Completed
            (Audio|PlaySoundatLocation "/Game/FancyApp/Audio/Open.Open" (Transformation|GetWorldLocation (Variables|Default|GetSM_RoomTumb_02)) "0, 0, 0" 1.0 1.0 0.0 "/Game/FancyApp/Audio/SA_Drawer.SA_Drawer" 0 0 0))))
      (:then_1
        (Utilities|FlowControl|DoOnce false) ; enters at Reset
      ))))

(event OnComponentEndOverlap(Sphere_Top)
  (params (OverlappedComponent :type Primitive%20Component%20Object%20Reference) (OtherActor :type Actor%20Object%20Reference) (OtherComp :type Primitive%20Component%20Object%20Reference) (OtherBodyIndex :type Integer))
  ;[0.15 0.15 0.15 0.5] TopDrawerPart_Sound
  (if (Components|ComponentHasTag OtherComp "TopCollision")
    (Utilities|FlowControl|Sequence
      (:then_0
        (Utilities|FlowControl|DoOnce false
          (:Completed
            (Audio|PlaySoundatLocation "/Game/FancyApp/Audio/Close.Close" (Transformation|GetWorldLocation (Variables|Default|GetSM_RoomTumb_02)) "0, 0, 0" 1.0 1.0 0.0 "/Game/FancyApp/Audio/SA_Drawer.SA_Drawer" 0 0 0))))
      (:then_1
        (Utilities|FlowControl|DoOnce false) ; enters at Reset
      ))))

(fn ConstructionScript)

(fn BoxTopper
  (bind _spline (Variables|Default|GetSpline))
  (bind _sphere_top (Variables|Default|GetSphere_Top))
  (bind _relativelocation (Variables|/Script/Engine.SceneComponent|GetRelativeLocation _sphere_top))
  (Transformation|SetRelativeLocation _sphere_top (Math|Vector|MakeVector (.x _relativelocation) (Math|Float|Clamp(Float) (+ (.y _relativelocation) (.y (.location (Math|Transform|MakeRelativeTransform (Transformation|GetWorldTransform (Variables|Default|GetMotion%20Controller)) (Transformation|GetWorldTransform (Variables|Default|GetSphere_Top)))))) (.y (Spline|GetLocationatSplinePoint _spline 0 "Local")) (.y (Spline|GetLocationatSplinePoint _spline 1 "Local"))) (.z _relativelocation)) false false))

(fn BoxDown
  (bind _sphere_bottom (Variables|Default|GetSphere_Bottom))
  (bind _spline (Variables|Default|GetSpline))
  (bind _relativelocation (Variables|/Script/Engine.SceneComponent|GetRelativeLocation _sphere_bottom))
  (Transformation|SetRelativeLocation _sphere_bottom (Math|Vector|MakeVector (.x _relativelocation) (Math|Float|Clamp(Float) (+ (.y _relativelocation) (.y (.location (Math|Transform|MakeRelativeTransform (Transformation|GetWorldTransform (Variables|Default|GetMotion%20Controller)) (Transformation|GetWorldTransform (Variables|Default|GetSphere_Bottom)))))) (.y (Spline|GetLocationatSplinePoint _spline 0 "Local")) (.y (Spline|GetLocationatSplinePoint _spline 1 "Local"))) (.z _relativelocation)) false false))