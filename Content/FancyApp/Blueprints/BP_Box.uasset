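; VR box Blueprint with a top piece that the player slides open by hand along one axis.
; On grab, it records the pawn's right grip controller position and the piece's relative location, regardless of which hand grabbed.
; Tick adds the controller's world Y movement to relative Y, clamped from zero to the open distance per grab, so it only slides one way.
; Dropping stops tracking; debug prints remain, and a timer-driven path is unused.
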(event OnGrabbed(GrabComponent_Top)
  (params (MotionController :type Motion%20Controller%20Component%20Object%20Reference))
  (bind _output_get (Variables|Default|SetGrabberPawn (.AsVRPawn (Utilities|Casting|CastToVRPawn (Game|Player|GetPlayerPawn 0)))))
  (bind _output_get_2 (Variables|Default|SetMotion%20Controller (Variables|/Game/VRTemplate/Blueprints/VRPawn.VRPawn_C|GetMotionControllerRightGrip _output_get)))
  (Utilities|IsValid _output_get_2
    (:Is%20Valid
      (Development|PrintString "IsValid" true true "(R=0.000000,G=0.660000,B=1.000000,A=1.000000)" 1e+01)
      (Variables|Default|SetbTopHeld true)
      (bind _output_get_3 (Variables|Default|SetMotion%20Controller MotionController))
      (Variables|Default|SetTop_StartControllerLoc (Transformation|GetWorldLocation _output_get_3))
      (Variables|Default|SetTop_StartDrawerRelLoc (Variables|/Script/Engine.SceneComponent|GetRelativeLocation (Variables|Default|GetSM_RoomTumb_02))))))

(event OnDropped(GrabComponent_Top)
  (Variables|Default|SetbTopHeld false)
  (Variables|Default|SetMotion%20Controller 0)
  (Development|PrintString "ONDROPPPPPPEDONDROPPPPPPEDONDROPPPPPPEDONDROPPPPPPEDONDROPPPPPPEDONDROPPPPPPEDONDROPPPPPPEDONDROPPPPPPEDONDROPPPPPPEDONDROPPPPPPEDONDROPPPPPPEDONDROPPPPPPEDONDROPPPPPPEDONDROPPPPPPEDONDROPPPPPPEDONDROPPPPPPEDONDROPPPPPPEDONDROPPPPPPEDONDROPPPPPPEDONDROPPPPPPEDONDROPPPPPPEDONDROPPPPPPEDONDROPPPPPPEDONDROPPPPPPEDONDROPPPPPPEDONDROPPPPPPEDONDROPPPPPPEDONDROPPPPPPEDONDROPPPPPPEDONDROPPPPPPEDONDROPPPPPPEDONDROPPPPPPEDONDROPPPPPPEDONDROPPPPPPEDONDROPPPPPPEDONDROPPPPPPEDONDROPPPPPPEDONDROPPPPPPEDONDROPPPPPPEDONDROPPPPPPEDONDROPPPPPPEDONDROPPPPPPEDONDROPPPPPPEDONDROPPPPPPEDONDROPPPPPPEDONDROPPPPPPEDONDROPPPPPPEDONDROPPPPPPEDONDROPPPPPPED" true true "(R=1.000000,G=0.923120,B=0.000000,A=1.000000)"))

(event Custom|TopBox)

(event EventTick
  (params (DeltaSeconds :type Float%20%28single-precision%29))
  (bind _top_startdrawerrelloc (Variables|Default|GetTop_StartDrawerRelLoc))
  (bind (_x _y _z) (Math|Vector|BreakVector _top_startdrawerrelloc))
  (Utilities|IsValid (Variables|Default|GetMotion%20Controller)
    (:Is%20Valid
      (if (Variables|Default|GetbTopHeld)
        (Transformation|SetRelativeLocation (Variables|Default|GetSM_RoomTumb_02) (Math|Vector|MakeVector _x (+ _y (Math|Float|Clamp(Float) (.y (- (Transformation|GetWorldLocation (Variables|Default|GetMotion%20Controller)) (Variables|Default|GetTop_StartControllerLoc))) 0.0 (Variables|Default|GetTop_OpenDistance))) _z) false false)))))

(fn ConstructionScript)