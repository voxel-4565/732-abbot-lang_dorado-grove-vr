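; Bathroom mirror actor that fakes a reflection by steering a SceneCaptureComponent2D from the player camera's position.
; A looping BeginPlay timer turns the camera's local-space position into a look-at from the root's world location, scales, inverts and clamps it, then captures manually.
; VRPawn box overlaps appear meant to throttle updates, but begin assigns the interval to itself and end's new value never reaches the running timer.
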(event OnComponentBeginOverlap(Box)
  (params (OverlappedComponent :type Primitive%20Component%20Object%20Reference) (OtherActor :type Actor%20Object%20Reference) (OtherComp :type Primitive%20Component%20Object%20Reference) (OtherBodyIndex :type Integer) (bFromSweep :type Boolean) (SweepResult :type Hit%20Result%20Structure%20%28by%20ref%29))
  (Utilities|Casting|CastToVRPawn OtherActor)
  (Variables|Default|SetTimeMirrorBathroomUpdate (Variables|Default|GetTimeMirrorBathroomUpdate)))

(event OnComponentEndOverlap(Box)
  (params (OverlappedComponent :type Primitive%20Component%20Object%20Reference) (OtherActor :type Actor%20Object%20Reference) (OtherComp :type Primitive%20Component%20Object%20Reference) (OtherBodyIndex :type Integer))
  (Utilities|Casting|CastToVRPawn OtherActor)
  (Variables|Default|SetTimeMirrorBathroomUpdate 25.0))

(event Custom|MirrorUpdateBathroom
  (bind _returnvalue (Game|GetPlayerCameraManager 0))
  (bind _defaultsceneroot (Variables|Default|GetDefaultSceneRoot))
  (bind _defaultsceneroot_2 (Variables|Default|GetDefaultSceneRoot))
  (bind _returnvalue_2 (Camera|GetCameraLocation _returnvalue))
  (bind _returnvalue_3 (Transformation|GetWorldTransform _defaultsceneroot_2))
  (bind _returnvalue_4 (Transformation|GetWorldLocation _defaultsceneroot))
  (bind _returnvalue_5 (Math|Transform|InverseTransformLocation _returnvalue_3 _returnvalue_2))
  (bind (_x _y _z) (Math|Vector|BreakVector _returnvalue_5))
  (bind _returnvalue_6 (Math|Vector|MakeVector _x _y _z))
  (bind _returnvalue_7 (Math|Rotator|FindLookatRotation _returnvalue_4 _returnvalue_6))
  (bind (_roll _pitch _yaw) (Math|Rotator|BreakRotator _returnvalue_7))
  (bind _returnvalue_8 (* _roll -1.0))
  (bind _returnvalue_9 (* _yaw -0.05))
  (bind _returnvalue_10 (* _pitch -0.5))
  (bind _returnvalue_11 (Math|Float|Clamp(Float) _returnvalue_10 -1e+01 4e+01))
  (bind _returnvalue_12 (Math|Float|Clamp(Float) _returnvalue_8 -2e+01 2e+01))
  (bind _returnvalue_13 (Math|Float|Clamp(Float) _returnvalue_9 -1.8e+02 1.8e+02))
  (bind _returnvalue_14 (Math|Rotator|MakeRotator _returnvalue_12 _returnvalue_11 _returnvalue_13))
  (Transformation|SetRelativeRotation (Variables|Default|GetSceneCaptureComponent2D) (Math|Rotator|MakeRotator (.roll _returnvalue_14) (.pitch _returnvalue_14) (.yaw _returnvalue_14)) false false)
  (Rendering|SceneCapture|CaptureScene (Variables|Default|GetSceneCaptureComponent2D) :!class /Script/Engine.SceneCaptureComponent2D))

(event EventBeginPlay
  (Utilities|Time|SetTimerbyEvent (delegate Custom|MirrorUpdateBathroom) (Variables|Default|GetTimeMirrorBathroomUpdate) true))

(fn ConstructionScript)