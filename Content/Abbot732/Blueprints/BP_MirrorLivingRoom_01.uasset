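; Living room mirror Blueprint that fakes a reflection by rotating a scene capture based on the player camera's position.
; A looping timer takes a look-at rotation from the mirror root to the camera's root-local position, then negates and clamps pitch and yaw.
; VR pawn overlaps write the update interval, but begin reassigns its current value, end sets a fixed one, and neither restarts the timer.
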(event OnComponentBeginOverlap(Box)
  (params (OverlappedComponent :type Primitive%20Component%20Object%20Reference) (OtherActor :type Actor%20Object%20Reference) (OtherComp :type Primitive%20Component%20Object%20Reference) (OtherBodyIndex :type Integer) (bFromSweep :type Boolean) (SweepResult :type Hit%20Result%20Structure%20%28by%20ref%29))
  (Utilities|Casting|CastToVRPawn OtherActor)
  (Variables|Default|SetTimeMirrorUpdate (Variables|Default|GetTimeMirrorUpdate)))

(event OnComponentEndOverlap(Box)
  (params (OverlappedComponent :type Primitive%20Component%20Object%20Reference) (OtherActor :type Actor%20Object%20Reference) (OtherComp :type Primitive%20Component%20Object%20Reference) (OtherBodyIndex :type Integer))
  (Utilities|Casting|CastToVRPawn OtherActor)
  (Variables|Default|SetTimeMirrorUpdate 15.0))

(event Custom|MirrorUpdate
  (bind _returnvalue (Game|GetPlayerCameraManager 0))
  (bind _defaultsceneroot (Variables|Default|GetDefaultSceneRoot))
  (bind _defaultsceneroot_2 (Variables|Default|GetDefaultSceneRoot))
  (bind _returnvalue_2 (Camera|GetCameraLocation _returnvalue))
  (bind _returnvalue_3 (Transformation|GetWorldTransform _defaultsceneroot_2))
  (bind _returnvalue_4 (Transformation|GetWorldLocation _defaultsceneroot))
  (bind _returnvalue_5 (Math|Transform|InverseTransformLocation _returnvalue_3 _returnvalue_2))
  (bind _returnvalue_6 (Math|Rotator|FindLookatRotation _returnvalue_4 _returnvalue_5))
  (bind (_roll _pitch _yaw) (Math|Rotator|BreakRotator _returnvalue_6))
  (Transformation|SetRelativeRotation (Variables|Default|GetSceneCaptureComponent2D) (Math|Rotator|MakeRotator _roll (Math|Float|Clamp(Float) (* _pitch -1.0) -45.0 45.0) (Math|Float|Clamp(Float) (* _yaw -1.0) -1.2e+02 1.2e+02)) false false))

(event EventBeginPlay
  (Utilities|Time|SetTimerbyEvent (delegate Custom|MirrorUpdate) (Variables|Default|GetTimeMirrorUpdate) true))

(fn ConstructionScript)