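; BP_MirrorLivingRoom1 is a fake mirror that uses a SceneCaptureComponent2D, with its Plane hidden from the capture.
; A looping timer moves the capture from the player camera's reflection about MirrorPlaneRoot, captures, then turns it along the mirror-to-camera direction.
; VRPawn leaving the Box sets TimeUpdateMirror to 10, but the timer is never restarted and entering reassigns the variable to itself.
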(event OnComponentBeginOverlap(Box)
  (params (OverlappedComponent :type Primitive%20Component%20Object%20Reference) (OtherActor :type Actor%20Object%20Reference) (OtherComp :type Primitive%20Component%20Object%20Reference) (OtherBodyIndex :type Integer) (bFromSweep :type Boolean) (SweepResult :type Hit%20Result%20Structure%20%28by%20ref%29))
  (Utilities|Casting|CastToVRPawn OtherActor)
  (Variables|Default|SetTimeUpdateMirror (Variables|Default|GetTimeUpdateMirror)))

(event OnComponentEndOverlap(Box)
  (params (OverlappedComponent :type Primitive%20Component%20Object%20Reference) (OtherActor :type Actor%20Object%20Reference) (OtherComp :type Primitive%20Component%20Object%20Reference) (OtherBodyIndex :type Integer))
  (Utilities|Casting|CastToVRPawn OtherActor)
  (Variables|Default|SetTimeUpdateMirror 1e+01))

(event Custom|UpdateImageMirror
  (bind _returnvalue (Game|GetPlayerCameraManager 0))
  (bind _mirrorplaneroot (Variables|Default|GetMirrorPlaneRoot))
  (bind _returnvalue_2 (Transformation|GetWorldLocation _mirrorplaneroot))
  (bind _returnvalue_3 (Math|Vector|GetForwardVector _mirrorplaneroot))
  (Utilities|FlowControl|Sequence
    (:then_0
      (bind _output_get (Variables|Default|SetCameraLocation (Camera|GetCameraLocation _returnvalue)))
      (bind _output_get_2 (Variables|Default|SetCameraRoration (Camera|GetCameraRotation _returnvalue)))
      (Transformation|SetWorldLocation (Variables|Default|GetSceneCaptureComponent2D) (/ (Math|Vector|MakeVector (.x (Math|Vector|NegateVector (Math|Vector|MakeVector (.X (Math|Vector|BreakVector (+ _returnvalue_3 (Math|Vector|GetReflectionVector (- _output_get _returnvalue_2) _returnvalue_3)))) 0.0 0.0))) (.Y (Math|Vector|BreakVector (+ _returnvalue_3 (Math|Vector|GetReflectionVector (- _output_get _returnvalue_2) _returnvalue_3)))) 3e+02) 2.0) false false)
      (Rendering|SceneCapture|CaptureScene (Variables|Default|GetSceneCaptureComponent2D) :!class /Script/Engine.SceneCaptureComponent2D)
      (Transformation|SetWorldRotation (Variables|Default|GetSceneCaptureComponent2D) (Math|Rotator|MakeRotator (.roll (Math|Rotator|FindLookatRotation _returnvalue_2 _output_get)) (.pitch (Math|Rotator|FindLookatRotation _returnvalue_2 _output_get)) (.yaw (Math|Rotator|FindLookatRotation _returnvalue_2 _output_get))) false false))))

(event EventBeginPlay
  (Utilities|FlowControl|Sequence
    (:then_0
      ;[0.15 0.15 0.15 0.5] FixBlackFrameBehind
      (Class|SceneCaptureComponent|HideComponent (Variables|Default|GetSceneCaptureComponent2D) (Variables|Default|GetPlane)))
    (:then_1
      (Utilities|Time|SetTimerbyEvent (delegate Custom|UpdateImageMirror) (Variables|Default|GetTimeUpdateMirror) true))))

(fn ConstructionScript)