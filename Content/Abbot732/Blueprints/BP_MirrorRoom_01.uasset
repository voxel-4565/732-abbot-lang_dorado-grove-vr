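; Mirror room actor for a VR game that fakes a reflection with a scene capture refreshed on a looping timer.
; While the VR pawn is inside the box trigger, the capture slides along local X, mapped from the player camera's Y relative to the mirror mesh.
; Overlap events set the inside flag and interval variable, but the running timer never picks up interval changes.
; Look-at rotation logic is left unused.
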(event OnComponentBeginOverlap(Box)
  (params (OverlappedComponent :type Primitive%20Component%20Object%20Reference) (OtherActor :type Actor%20Object%20Reference) (OtherComp :type Primitive%20Component%20Object%20Reference) (OtherBodyIndex :type Integer) (bFromSweep :type Boolean) (SweepResult :type Hit%20Result%20Structure%20%28by%20ref%29))
  (Utilities|Casting|CastToVRPawn OtherActor)
  (Variables|Default|SetIsPlayerInside true)
  (Variables|Default|SetTimeMirrorRoomUpdate (Variables|Default|GetTimeMirrorRoomUpdate)))

(event OnComponentEndOverlap(Box)
  (params (OverlappedComponent :type Primitive%20Component%20Object%20Reference) (OtherActor :type Actor%20Object%20Reference) (OtherComp :type Primitive%20Component%20Object%20Reference) (OtherBodyIndex :type Integer))
  (Utilities|Casting|CastToVRPawn OtherActor)
  (Variables|Default|SetIsPlayerInside false)
  (Variables|Default|SetTimeMirrorRoomUpdate (Variables|Default|GetTimeMirrorBathroomUpdate_AFK)))

(event Custom|MirrorUpdateBathroom
  (Rendering|SceneCapture|CaptureScene (Variables|Default|GetSceneCaptureComponent2D) :!class /Script/Engine.SceneCaptureComponent2D)
  (if (Variables|Default|GetIsPlayerInside)
    (Transformation|SetRelativeLocation (Variables|Default|GetSceneCaptureComponent2D) (Math|Vector|MakeVector (Math|Float|MapRangeClamped (.Y (Math|Vector|BreakVector (Math|Transform|InverseTransformLocation (Transformation|GetWorldTransform (Variables|Default|GetSM_MirrorLivingRoom_02)) (Camera|GetCameraLocation (Game|GetPlayerCameraManager 0))))) -28.0 -5e+02 0.0 1.3e+02) 0.0 0.0) false false)))

(event EventBeginPlay
  (Utilities|Time|SetTimerbyEvent (delegate Custom|MirrorUpdateBathroom) (Variables|Default|GetTimeMirrorRoomUpdate) true))

(fn ConstructionScript)