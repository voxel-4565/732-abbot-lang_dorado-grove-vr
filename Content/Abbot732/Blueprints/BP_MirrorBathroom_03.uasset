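; Bathroom mirror actor that fakes a reflection with a SceneCaptureComponent2D.
; A looping timer started at BeginPlay calls CaptureScene every TimeMirrorBathroomUpdate seconds.
; VRPawn box overlaps write that variable (self-assignment on enter, 25 on exit) but never restart the timer, so its rate stays fixed.
; Capture rotation logic and clamped camera look-at math remain unwired.
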(event OnComponentBeginOverlap(Box)
  (params (OverlappedComponent :type Primitive%20Component%20Object%20Reference) (OtherActor :type Actor%20Object%20Reference) (OtherComp :type Primitive%20Component%20Object%20Reference) (OtherBodyIndex :type Integer) (bFromSweep :type Boolean) (SweepResult :type Hit%20Result%20Structure%20%28by%20ref%29))
  (Utilities|Casting|CastToVRPawn OtherActor)
  (Variables|Default|SetTimeMirrorBathroomUpdate (Variables|Default|GetTimeMirrorBathroomUpdate)))

(event OnComponentEndOverlap(Box)
  (params (OverlappedComponent :type Primitive%20Component%20Object%20Reference) (OtherActor :type Actor%20Object%20Reference) (OtherComp :type Primitive%20Component%20Object%20Reference) (OtherBodyIndex :type Integer))
  (Utilities|Casting|CastToVRPawn OtherActor)
  (Variables|Default|SetTimeMirrorBathroomUpdate 25.0))

(event Custom|MirrorUpdateBathroom
  (Rendering|SceneCapture|CaptureScene (Variables|Default|GetSceneCaptureComponent2D) :!class /Script/Engine.SceneCaptureComponent2D))

(event EventBeginPlay
  (Utilities|Time|SetTimerbyEvent (delegate Custom|MirrorUpdateBathroom) (Variables|Default|GetTimeMirrorBathroomUpdate) true))

(fn ConstructionScript)