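; Bathroom mirror for a VR level, faking a reflection with a manually triggered SceneCaptureComponent2D.
; A looping timer from BeginPlay updates the capture only while a VRPawn is inside the Box trigger.
; Each update slides the capture along Y from the camera's world X and applies a tightly clamped, inverted look-at pitch before capturing.
; Overlap events also write the interval variable, but never restart the timer.
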(event OnComponentBeginOverlap(Box)
  (params (OverlappedComponent :type Primitive%20Component%20Object%20Reference) (OtherActor :type Actor%20Object%20Reference) (OtherComp :type Primitive%20Component%20Object%20Reference) (OtherBodyIndex :type Integer) (bFromSweep :type Boolean) (SweepResult :type Hit%20Result%20Structure%20%28by%20ref%29))
  (Utilities|Casting|CastToVRPawn OtherActor)
  (Variables|Default|SetIsPlayerInside true)
  (Variables|Default|SetTimeMirrorBathroom2Update (Variables|Default|GetTimeMirrorBathroom2Update)))

(event OnComponentEndOverlap(Box)
  (params (OverlappedComponent :type Primitive%20Component%20Object%20Reference) (OtherActor :type Actor%20Object%20Reference) (OtherComp :type Primitive%20Component%20Object%20Reference) (OtherBodyIndex :type Integer))
  (Utilities|Casting|CastToVRPawn OtherActor)
  (Variables|Default|SetIsPlayerInside false)
  (Variables|Default|SetTimeMirrorBathroom2Update 25.0))

(event Custom|MirrorUpdateBathroom
  (bind _returnvalue (Game|GetPlayerCameraManager 0))
  (bind _defaultsceneroot (Variables|Default|GetDefaultSceneRoot))
  (bind _defaultsceneroot_2 (Variables|Default|GetDefaultSceneRoot))
  (bind _scenecapturecomponent2d (Variables|Default|GetSceneCaptureComponent2D))
  (bind _returnvalue_2 (Camera|GetCameraLocation _returnvalue))
  (bind _returnvalue_3 (Transformation|GetWorldTransform _defaultsceneroot_2))
  (bind _returnvalue_4 (Transformation|GetWorldLocation _defaultsceneroot))
  (bind _relativelocation (Variables|/Script/Engine.SceneComponent|GetRelativeLocation _scenecapturecomponent2d))
  (bind _returnvalue_5 (Math|Transform|InverseTransformLocation _returnvalue_3 _returnvalue_2))
  (bind (_x _y _z) (Math|Vector|BreakVector _returnvalue_5))
  (bind _returnvalue_6 (Math|Vector|MakeVector _x _y _z))
  (bind _returnvalue_7 (Math|Rotator|FindLookatRotation _returnvalue_4 _returnvalue_6))
  (bind _pitch (Math|Rotator|BreakRotator _returnvalue_7))
  (bind _returnvalue_8 (* _pitch -1.0))
  (bind _returnvalue_9 (Math|Float|Clamp(Float) _returnvalue_8 -1.0))
  (bind _returnvalue_10 (Math|Rotator|MakeRotator 0.0 _returnvalue_9 0.0))
  (if (Variables|Default|GetIsPlayerInside)
    (Transformation|SetRelativeLocation (Variables|Default|GetSceneCaptureComponent2D) (Math|Vector|MakeVector (.x _relativelocation) (.Y (Math|Vector|BreakVector (* (Math|Float|MapRangeClamped (.X (Math|Vector|BreakVector (Transformation|GetActorLocation (Game|GetPlayerCameraManager 0)))) -2.5e+02 6.5e+02 -2e+02 2e+02) 0.5))) (.z _relativelocation)) false false)
    (Transformation|SetRelativeRotation (Variables|Default|GetSceneCaptureComponent2D) (Math|Rotator|MakeRotator (.roll _returnvalue_10) (.pitch _returnvalue_10) (.yaw _returnvalue_10)) false false)
    (Rendering|SceneCapture|CaptureScene (Variables|Default|GetSceneCaptureComponent2D) :!class /Script/Engine.SceneCaptureComponent2D)))

(event EventBeginPlay
  (Utilities|Time|SetTimerbyEvent (delegate Custom|MirrorUpdateBathroom) (Variables|Default|GetTimeMirrorBathroom2Update) true))

(fn ConstructionScript)