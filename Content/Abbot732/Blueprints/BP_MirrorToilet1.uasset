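; BP_MirrorToilet1 is a mirror whose reflection comes from a scene capture component that hides the SMMirror02 mesh from its own view.
; A looping timer refreshes the capture manually, using the TimeUpdateMirror interval read at BeginPlay.
; VRPawn box overlaps write that interval, but entry assigns it to itself and exit's longer value never restarts the running timer.
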(event OnComponentBeginOverlap(Box)
  (params (OverlappedComponent :type Primitive%20Component%20Object%20Reference) (OtherActor :type Actor%20Object%20Reference) (OtherComp :type Primitive%20Component%20Object%20Reference) (OtherBodyIndex :type Integer) (bFromSweep :type Boolean) (SweepResult :type Hit%20Result%20Structure%20%28by%20ref%29))
  (Utilities|Casting|CastToVRPawn OtherActor)
  (Variables|Default|SetTimeUpdateMirror (Variables|Default|GetTimeUpdateMirror)))

(event OnComponentEndOverlap(Box)
  (params (OverlappedComponent :type Primitive%20Component%20Object%20Reference) (OtherActor :type Actor%20Object%20Reference) (OtherComp :type Primitive%20Component%20Object%20Reference) (OtherBodyIndex :type Integer))
  (Utilities|Casting|CastToVRPawn OtherActor)
  (Variables|Default|SetTimeUpdateMirror 1e+01))

(event Custom|UpdateMirror
  (Rendering|SceneCapture|CaptureScene (Variables|Default|GetSceneCaptureComponent2D) :!class /Script/Engine.SceneCaptureComponent2D))

(event EventBeginPlay
  (Utilities|FlowControl|Sequence
    (:then_0
      (Class|SceneCaptureComponent|HideComponent (Variables|Default|GetSceneCaptureComponent2D) (Variables|Default|GetSM_Mirror_02)))
    (:then_1
      (Utilities|Time|SetTimerbyEvent (delegate Custom|UpdateMirror) (Variables|Default|GetTimeUpdateMirror) true))))

(fn ConstructionScript)